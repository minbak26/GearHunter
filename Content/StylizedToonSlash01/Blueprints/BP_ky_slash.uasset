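; Demo actor for stylized toon slash effects that plays a looping three-slash sequence from BeginPlay.
; Chained timelines and delays roll the Scene component between slashes and pitch the Pivot through each swing, triggering paired FX and NS effects.
; IsHitFX also fires matching hit effects for each slash.
; A final timeline resets both rotations before jumping back to the start; Tick and overlap events are unused.
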(event EventBeginPlay
  ;[1 1 1] set rotation
  (Components|Activation|Deactivate (Variables|Default|GetFX1))
  (Transformation|SetRelativeRotation (Variables|Default|GetScene) (Math|Rotator|MakeRotator 45.0 0.0 0.0) false false :!label _label)
  (bind _y (Timeline|Timeline_0 PlayFromStart)
    (:Update
      (Transformation|SetRelativeRotation (Variables|Default|Getpivot) (Math|Rotator|MakeRotator 0.0 _y 0.0) false false)
      ;[1 1 1] effect control
      (Utilities|FlowControl|Delay 0.1)
      (Components|Activation|Activate (Variables|Default|GetFX1) false)
      (if (Variables|Default|GetisHitFX)
        (Components|Activation|Activate (Variables|Default|GetSlashHit1) false))
      (Utilities|FlowControl|Delay 0.3)
      ;[1 1 1] control rot
      (bind _newtrack_0 (Timeline|Timeline_2 PlayFromStart)
        (:Update
          (Transformation|SetRelativeRotation (Variables|Default|GetScene) (Math|Rotator|MakeRotator _newtrack_0 0.0 0.0) false false)
          (Utilities|FlowControl|Delay 0.2)
          (bind _newtrack_0_2 (Timeline|Timeline_1 PlayFromStart)
            (:Update
              (Transformation|SetRelativeRotation (Variables|Default|Getpivot) (Math|Rotator|MakeRotator 0.0 _newtrack_0_2 0.0) false false)
              ;[1 1 1] fx control
              (Utilities|FlowControl|Delay 0.05)
              (Components|Activation|Activate (Variables|Default|GetFX2) false)
              (if (Variables|Default|GetisHitFX)
                (Components|Activation|Activate (Variables|Default|GetSlashHit2) false))
              (Utilities|FlowControl|Delay 0.3)
              ;[1 1 1] slash3 control
              (bind _newtrack_0_3 (Timeline|Timeline_3 PlayFromStart)
                (:Update
                  (Transformation|SetRelativeRotation (Variables|Default|GetScene) (Math|Rotator|MakeRotator _newtrack_0_3 0.0 0.0) false false)
                  (Utilities|FlowControl|Delay 0.3)
                  (bind _newtrack_0_4 (Timeline|Timeline_4 PlayFromStart)
                    (:Update
                      (Transformation|SetRelativeRotation (Variables|Default|Getpivot) (Math|Rotator|MakeRotator 0.0 _newtrack_0_4 0.0) false false)
                      (Utilities|FlowControl|Delay 0.1)
                      (Components|Activation|Activate (Variables|Default|GetFX3) false)
                      (if (Variables|Default|GetisHitFX)
                        (Components|Activation|Activate (Variables|Default|GetSlashHit3) false))
                      (Utilities|FlowControl|Delay 0.6)
                      ;[1 1 1] init
                      (bind (_direction _newtrack_0_5 _newtrack_2) (Timeline|Timeline_5 PlayFromStart)
                        (:Update
                          (Transformation|SetRelativeRotation (Variables|Default|GetScene) (Math|Rotator|MakeRotator _newtrack_0_5 0.0 0.0) false false)
                          (Transformation|SetRelativeRotation (Variables|Default|Getpivot) (Math|Rotator|MakeRotator 0.0 _newtrack_2 0.0) false false)
                          (Utilities|FlowControl|Delay 0.3)
                          (goto _label))))))))))))))

(event Collision|EventActorBeginOverlap
  (params (OtherActor :type Actor%20Object%20Reference)))

(event EventTick
  (params (DeltaSeconds :type Float%20%28single-precision%29)))

(fn ConstructionScript)