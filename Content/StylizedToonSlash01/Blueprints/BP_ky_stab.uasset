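; BP_ky_stab is an effect actor that plays a looping stab motion with stab and hit FX, apparently as a showcase.
; On BeginPlay a timeline drives the Pivot along X, while a delay chain from its update fires stab FX, then hit FX, and restarts the cycle.
; Regular and NS-prefixed FX activate together, as the UseNiagara branch is unconnected.
; The construction script applies X offsets to the effects.
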(event EventBeginPlay
  ;[1 1 1] init
  (Rendering|SetVisibility (Variables|Default|GetStaticMesh) (Variables|Default|GetisMeshVisible) false)
  (Components|Activation|Deactivate (Variables|Default|GetStabFX))
  ;[1 1 1] fx control
  (bind _xvalue (Timeline|Timeline_0 PlayFromStart)
    (:Update
      (Transformation|SetRelativeLocation (Variables|Default|GetPivot) (Math|Vector|MakeVector _xvalue 0.0 0.0) false false)
      (Utilities|FlowControl|Delay 0.1)
      (Components|Activation|Activate (Variables|Default|GetStabFX) false)
      (Utilities|FlowControl|Delay 0.05)
      (Components|Activation|Activate (Variables|Default|GetStabHitFX) false)
      (Utilities|FlowControl|Delay 1.0)
      (Components|Activation|Deactivate (Variables|Default|GetStabFX))
      (Timeline|Timeline_0 PlayFromStart))))

(event Collision|EventActorBeginOverlap
  (params (OtherActor :type Actor%20Object%20Reference)))

(event EventTick
  (params (DeltaSeconds :type Float%20%28single-precision%29)))

(fn ConstructionScript
  ;[1 1 1] fx offset
  (Transformation|SetRelativeLocation (Variables|Default|GetStabFX) (Math|Vector|MakeVector (Variables|Default|GetFxOfsX) 0.0 0.0) false false)
  (Transformation|SetRelativeLocation (Variables|Default|GetStabHitFX) (Math|Vector|MakeVector (Variables|Default|GetHitFxOfsX) 0.0 0.0) false false))